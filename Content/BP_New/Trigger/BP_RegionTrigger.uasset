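; Region trigger that spawns one actor of a configurable class just above itself when the count of BP_player_M actors in its Box is within Min–Max.
; The count is seeded on BeginPlay and updated by overlap events, but spawning is attempted only at start and on player entry.
; A flag prevents duplicate spawns; the spawned actor's OnDestroyed clears it without immediately respawning.
; GetModuleName returns a script module path.
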(event `self.ReceiveBeginPlay`
  (`|ExecutionSequence`
    (:`then_0`
      (`KismetSystemLibrary.Delay` 1.0)
      (`KismetSystemLibrary.PrintString` (`KismetStringLibrary.Concat_StrStr` "初始玩家数" (`KismetStringLibrary.Conv_IntToString` (`GameplayStatics.GetNumPlayerControllers`)))))
    (:`then_1`
      (set `self.区域内玩家数` (`KismetArrayLibrary.Array_Length` (`PrimitiveComponent.GetOverlappingActors` (`self.Box`) "/Game/BP_New/BP_player_M.BP_player_M_C")))
      (`self.尝试生成` :!label _label))))

(event `self.ReceiveTick`
  (params (DeltaSeconds :type "Float (single-precision)"))
  (`parent.ReceiveTick` 0.0))

(event `self.Box.OnComponentBeginOverlap`
  (params (OverlappedComponent :type "PrimitiveComponent Object Reference") (OtherActor :type "Actor Object Reference") (OtherComp :type "PrimitiveComponent Object Reference") (OtherBodyIndex :type Integer) (bFromSweep :type Boolean) (SweepResult :type "HitResult Structure (by ref)"))
  (cast `/Game/BP_New/BP_player_M` OtherActor)
  (`/Engine/EditorBlueprintResources/StandardMacros.IncrementInt` (`self.区域内玩家数`)
    (:`  `
      (goto _label))))

(event `self.Box.OnComponentEndOverlap`
  (params (OverlappedComponent :type "PrimitiveComponent Object Reference") (OtherActor :type "Actor Object Reference") (OtherComp :type "PrimitiveComponent Object Reference") (OtherBodyIndex :type Integer))
  (cast `/Game/BP_New/BP_player_M` OtherActor)
  (`/Engine/EditorBlueprintResources/StandardMacros.DecrementInt` (`self.区域内玩家数`)))

(event `尝试生成`
  (if (`self.生成条件判断`)
    (if (not (`self.已生成完成`))
      (bind _returnvalue (`|SpawnActorFromClass` (`self.Class`) (`KismetMathLibrary.Conv_VectorToTransform` (+ (`self.K2_GetActorLocation`) (0.0 0.0 100.0))) "Undefined" "MultiplyWithRoot" null null))
      (`/Engine/EditorBlueprintResources/StandardMacros.IsValid` _returnvalue
        (:`Is Valid`
          (set `self.已生成完成` true)
          (add `self.OnDestroyed` _returnvalue (delegate `销毁时重置`)))))))

(event `销毁时重置` :!signature `self.OnDestroyed`
  (params (DestroyedActor :type "Actor Object Reference"))
  (set `self.已生成完成` false))

(fn `GetModuleName`
  (returns (ReturnValue :type String))
  (return "BP_New.Trigger.BP_RegionTrigger_C"))

(fn `UserConstructionScript`)

(fn `生成条件判断`
  (returns (ReturnValue :type Boolean))
  (return (`KismetMathLibrary.InRange_IntInt` (`self.区域内玩家数`) (`self.Min`) (`self.Max`))))