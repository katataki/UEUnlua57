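; BP_Spawner is a trigger actor that spawns a BP_MonsterCharacter at its own transform whenever a Pawn overlaps its Box.
; A player-count check chooses between a normal spawn owned by that pawn and an ownerless one with doubled scale.
; The GetNumPlayers call feeding that check is never executed, so the count is not actually refreshed from the game mode.
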(event OnComponentBeginOverlap(Box)
  (params (OverlappedComponent :type Primitive%20Component%20Object%20Reference) (OtherActor :type Actor%20Object%20Reference) (OtherComp :type Primitive%20Component%20Object%20Reference) (OtherBodyIndex :type Integer) (bFromSweep :type Boolean) (SweepResult :type Hit%20Result%20Structure%20%28by%20ref%29))
  (bind _aspawn (Utilities|Casting|CastToPawn OtherActor))
  (if (== (stale _returnvalue) 0)
    (Game|SpawnActorfromClass "/Game/Blueprint/Monster/BP_MonsterCharacter.BP_MonsterCharacter_C" (Transformation|GetActorTransform) "Undefined" "MultiplyWithRoot" _aspawn 0)
    (else
      (Game|SpawnActorfromClass "/Game/Blueprint/Monster/BP_MonsterCharacter.BP_MonsterCharacter_C" (Math|Transform|ComposeTransforms (Transformation|GetActorTransform) (Math|Transform|MakeTransform "0, 0, 0" "0, 0, 0" "2.000000,2.000000,2.000000")) "Undefined" "MultiplyWithRoot" 0 0))))

(event EventBeginPlay)

(event Collision|EventActorBeginOverlap
  (params (OtherActor :type Actor%20Object%20Reference)))

(event EventTick
  (params (DeltaSeconds :type Float%20%28single-precision%29)))

(fn ConstructionScript)