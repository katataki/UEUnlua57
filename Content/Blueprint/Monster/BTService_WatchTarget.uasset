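; Behavior tree service that keeps a monster's target and its distance to that target current on the blackboard.
; Each AI tick, a valid Target has its straight-line distance from the controlled pawn written to DistanceToTarget.
; Without one, it stores the first BP_player_M actor found through TargetKey and measures that distance.
; If no player exists, it clears TargetKey and writes a very large fallback distance.
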(event `self.ReceiveTickAI`
  (params (OwnerController :type "AIController Object Reference") (ControlledPawn :type "Pawn Object Reference") (DeltaSeconds :type "Float (single-precision)"))
  (bind _targetkey (`self.TargetKey`))
  (bind _returnvalue (`BTFunctionLibrary.GetBlackboardValueAsObject` (make `BlackboardKeySelector` :`SelectedKeyName` "Target")))
  (set `self.Controlled Pawn` ControlledPawn)
  (`/Engine/EditorBlueprintResources/StandardMacros.IsValid` _returnvalue
    (:`Is Valid`
      ; 更新到目标的距离
      (bind _asactor (cast `Actor` _returnvalue))
      (set `self.TargetActor` _asactor)
      (`BTFunctionLibrary.SetBlackboardValueAsFloat` (make `BlackboardKeySelector` :`SelectedKeyName` "DistanceToTarget") (`KismetMathLibrary.VSize` (- (`Actor.K2_GetActorLocation` (`self.TargetActor`)) (`Actor.K2_GetActorLocation` (`self.Controlled Pawn`))))))
    (:`Is Not Valid`
      ; 找玩家角色
      (bind _outactors (`GameplayStatics.GetAllActorsOfClass` "/Game/BP_New/BP_player_M.BP_player_M_C"))
      (if (> (`KismetArrayLibrary.Array_Length` _outactors) 0)
        (set `self.TargetActor` (`|GetArrayItem` _outactors))
        (`BTFunctionLibrary.SetBlackboardValueAsObject` _targetkey (`self.TargetActor`))
        ; 更新到目标的距离
        (`BTFunctionLibrary.SetBlackboardValueAsFloat` (make `BlackboardKeySelector` :`SelectedKeyName` "DistanceToTarget") (`KismetMathLibrary.VSize` (- (`Actor.K2_GetActorLocation` (`self.TargetActor`)) (`Actor.K2_GetActorLocation` (`self.Controlled Pawn`)))))
        (else
          ; 找不到假定目标在极远处
          (`BTFunctionLibrary.SetBlackboardValueAsObject` _targetkey)
          (`BTFunctionLibrary.SetBlackboardValueAsFloat` (make `BlackboardKeySelector` :`SelectedKeyName` "DistanceToTarget") 1000000.0))))))