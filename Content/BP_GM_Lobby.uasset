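; BP_GM_Lobby is a lobby game mode Blueprint with helpers for spawn placement, pawn cleanup and map settings.
; GetStartTransform returns the first PlayerStart's transform, and DestoryOld destroys a controller's current pawn if it is valid.
; SetMapName copies MapName and MaxPlayer from BP_GameInstance, and GetModuleName returns the class name as a string.
; The player-info add and update events and UpdateAllPlayer are empty stubs.
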(event `Event_UpdatePlayerInfo`
  (params (PlayerInfo :type "/Game/Blueprint/PlayerInfo Structure")))

(event `Event_AddPlayerInfo`
  (params (PlayerInfo :type "/Game/Blueprint/PlayerInfo Structure")))

(event `UpdateAllPlayer`)

(fn `DestoryOld`
  (params (Controller :type "PlayerController Object Reference"))
  (bind _returnvalue (`Controller.K2_GetPawn` Controller))
  (`/Engine/EditorBlueprintResources/StandardMacros.IsValid` _returnvalue
    (:`Is Valid`
      (`self.K2_DestroyActor` _returnvalue))))

(fn `GetModuleName`
  (returns (ReturnValue :type String))
  (return "BP_GM_Lobby_C"))

(fn `GetStartTransform`
  (returns (Trans :type "Transform Structure"))
  (bind _outactors (`GameplayStatics.GetAllActorsOfClass` "/Script/Engine.PlayerStart"))
  (return (`self.GetTransform` (`|GetArrayItem` _outactors))))

(fn `SetMapName`
  (bind _asbp_game_instance (cast `/Game/BP_GameInstance` (`GameplayStatics.GetGameInstance`)))
  (set `self.MapName` (`/Game/BP_GameInstance.MapName` _asbp_game_instance))
  (set `self.Max Player` (`/Game/BP_GameInstance.MaxPlayer` _asbp_game_instance)))

(fn `UserConstructionScript`)